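; TriggerButton is a button Blueprint that changes color and moves its Cube mesh when its custom events are called from outside the event graph.
; Material_Change creates a dynamic material instance, tints it green and plays a timeline that sets the Cube's relative location to LowerAmount scaled by the ButtonLower track.
; Material_Change_Reverse creates another instance with an overbright red tint and reverses the timeline.
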(event Custom|Material_Change_Reverse
  (bind _returnvalue (Rendering|Material|CreateDynamicMaterialInstance (Variables|Default|GetCube) 0 "/Game/Aesthetics/Materials/Button.Button" :!class /Script/Engine.PrimitiveComponent))
  (Rendering|Material|SetVectorParameterValue _returnvalue "Color" "(R=138.000000,G=6.999998,B=6.999998,A=0.500000)" :!class /Script/Engine.MaterialInstanceDynamic)
  (bind _buttonlower (Timeline|Timeline_0 Reverse)
    (:Update
      (Transformation|SetRelativeLocation (Variables|Default|GetCube) (* (stale Custom|Material_Change lowerAmount) _buttonlower) false false))))

(event Custom|Material_Change
  (params (lowerAmount :type Vector :default "0,0.000000,-15.000000"))
  (bind _returnvalue (Rendering|Material|CreateDynamicMaterialInstance (Variables|Default|GetCube) 0 "/Game/Aesthetics/Materials/Button.Button" :!class /Script/Engine.PrimitiveComponent))
  (Rendering|Material|SetVectorParameterValue _returnvalue "Color" "(R=0.000000,G=1.000000,B=0.094779,A=1.000000)" :!class /Script/Engine.MaterialInstanceDynamic)
  (bind _buttonlower (Timeline|Timeline_0 Play)
    (:Update
      (Transformation|SetRelativeLocation (Variables|Default|GetCube) (* lowerAmount _buttonlower) false false))))

(fn ConstructionScript)